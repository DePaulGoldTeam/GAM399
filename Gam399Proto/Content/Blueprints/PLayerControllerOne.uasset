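; First player controller that drives two characters from one controller's input, for a two-player setup.
; On BeginPlay it spawns a PlayerControllerTwo and a PlayerTwo at a fixed location, has that controller possess the character, and stores both references.
; MoveForward and MoveRight move its own pawn, while MoveForward2 and MoveRight2 move the second character directly, each relative to that pawn's control rotation.
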(event EventBeginPlay
  (bind _returnvalue (Math|Transform|MakeTransform "-900.000000,900.000000,230.000000" "0, 0, 0" "1,1,1.000000"))
  (bind _returnvalue_2 (Game|SpawnActorfromClass "/Game/Blueprints/PlayerControllerTwo.PlayerControllerTwo_C" _returnvalue false 0))
  (Variables|Default|SetMyplayercontroller _returnvalue_2)
  (bind _returnvalue_3 (Game|SpawnActorfromClass "/Game/Blueprints/PlayerTwo.PlayerTwo_C" _returnvalue false 0))
  (Variables|Default|SetCharacter2 _returnvalue_3)
  (Pawn|Possess (Variables|Default|GetMyplayercontroller) (Variables|Default|GetCharacter2)))

(event Input|AxisEvents|InputAxisMoveRight
  (params (AxisValue :type Float%20%28single-precision%29))
  (bind _returnvalue (Pawn|GetControlledPawn))
  (Pawn|Input|AddMovementInput _returnvalue (Math|Vector|GetRightVector (Pawn|GetControlRotation _returnvalue :!class /Script/Engine.Pawn)) AxisValue false))

(event Input|AxisEvents|InputAxisMoveForward2
  (params (AxisValue :type Float%20%28single-precision%29))
  (bind _character2 (Variables|Default|GetCharacter2))
  (Pawn|Input|AddMovementInput _character2 (Math|Vector|GetForwardVector (Pawn|GetControlRotation _character2 :!class /Script/Engine.Pawn)) AxisValue false))

(event Input|AxisEvents|InputAxisMoveRight2
  (params (AxisValue :type Float%20%28single-precision%29))
  (bind _character2 (Variables|Default|GetCharacter2))
  (Pawn|Input|AddMovementInput _character2 (Math|Vector|GetRightVector (Pawn|GetControlRotation _character2 :!class /Script/Engine.Pawn)) AxisValue false))

(event Input|AxisEvents|InputAxisMoveForward
  (params (AxisValue :type Float%20%28single-precision%29))
  (bind _returnvalue (Pawn|GetControlledPawn))
  (Pawn|Input|AddMovementInput _returnvalue (Math|Vector|GetForwardVector (Pawn|GetControlRotation _returnvalue :!class /Script/Engine.Pawn)) AxisValue false))

(fn ConstructionScript)